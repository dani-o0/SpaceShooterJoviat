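; Space shooter fire-rate power-up that lowers the player's FireDelay when overlapped by an SS_Player_Character.
; On pickup it destroys itself, then sets a 30-second timer by function name on itself for RevertFirerate, so the revert likely never fires.
; RevertFirerate looks up player character 0 and sets a hardcoded slower delay rather than restoring the previous value.
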(event `self.ReceiveActorBeginOverlap`
  (params (OtherActor :type "Actor Object Reference"))
  ; Comentario
  (bind _asss_player_character (cast `/Game/00_Space_Shooter/Player/SS_Player_Character` OtherActor))
  (set `/Game/00_Space_Shooter/Player/SS_Player_Character.Fire Delay` 0.2 _asss_player_character)
  (`self.K2_DestroyActor`)
  (`KismetSystemLibrary.K2_SetTimer` null "RevertFirerate" 30.0))

(fn `RevertFirerate`
  ; Comentario
  (bind _asss_player_character (cast `/Game/00_Space_Shooter/Player/SS_Player_Character` (`GameplayStatics.GetPlayerCharacter` 0)))
  (set `/Game/00_Space_Shooter/Player/SS_Player_Character.Fire Delay` 2.0 _asss_player_character))

(fn `UserConstructionScript`
  (`parent.UserConstructionScript`))