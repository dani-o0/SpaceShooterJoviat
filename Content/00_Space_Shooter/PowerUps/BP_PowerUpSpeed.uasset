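; BP_PowerUpSpeed is a speed power-up pickup for the space shooter.
; When an SS_Player_Character overlaps it, the actor destroys itself, with no speed boost applied in these graphs.
; A separate RevertSpeed function sets the Speed of player 0's character back to a hardcoded value, but nothing in this file calls it.
; BeginPlay and Tick are disabled parent-call stubs.
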(event `self.ReceiveActorBeginOverlap`
  (params (OtherActor :type "Actor Object Reference"))
  ; Comentario
  (cast `/Game/00_Space_Shooter/Player/SS_Player_Character` OtherActor)
  (`self.K2_DestroyActor`))

(fn `RevertSpeed`
  (bind _asss_player_character (cast `/Game/00_Space_Shooter/Player/SS_Player_Character` (`GameplayStatics.GetPlayerCharacter` 0)))
  (set `/Game/00_Space_Shooter/Player/SS_Player_Character.Speed` 500.0 _asss_player_character))

(fn `UserConstructionScript`
  (`parent.UserConstructionScript`))