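; BP_PowerUpBase is a space shooter power-up that drifts through the level and gives the player an extra life on contact.
; It caches its forward vector at BeginPlay and moves along it every Tick at Speed, scaled by delta time and without sweeping.
; Overlapping SS_Player_Character increments NumLifes unless it equals three, then destroys the pickup even if no life was added.
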(event `self.ReceiveBeginPlay`
  ; Comentario
  (set `self.MovementVector` (`self.GetActorForwardVector`)))

(event `self.ReceiveActorBeginOverlap`
  (params (OtherActor :type "Actor Object Reference"))
  ; Comentario
  (bind _asss_player_character (cast `/Game/00_Space_Shooter/Player/SS_Player_Character` OtherActor))
  (bind _numlifes (`/Game/00_Space_Shooter/Player/SS_Player_Character.NumLifes` _asss_player_character))
  (if (not (== _numlifes 3))
    (set `/Game/00_Space_Shooter/Player/SS_Player_Character.NumLifes` (+ _numlifes 1) _asss_player_character))
  (`self.K2_DestroyActor`))

(event `self.ReceiveTick`
  (params (DeltaSeconds :type "Float (single-precision)"))
  ; Comentario
  (`self.K2_SetActorLocation` (+ (`self.K2_GetActorLocation`) (* (* DeltaSeconds (`self.Speed`)) (`self.MovementVector`)))))

(fn `UserConstructionScript`)