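; BP_EnemyV is a space shooter enemy variant that faces the player every frame.
; It inherits begin play, overlap and tick behavior from its parent, and its construction script sets movement speed and shot delay.
; Tick feeds the look-at rotation toward player 0 into RInterpTo as Current, with Target and DeltaTime unset, so the turn snaps instead of easing.
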(event `self.ReceiveBeginPlay`
  (`parent.ReceiveBeginPlay`))

(event `self.ReceiveActorBeginOverlap`
  (params (OtherActor :type "Actor Object Reference"))
  (`parent.ReceiveActorBeginOverlap` OtherActor))

(event `self.ReceiveTick`
  (params (DeltaSeconds :type "Float (single-precision)"))
  (`parent.ReceiveTick` DeltaSeconds)
  (`self.K2_SetActorRotation` (`KismetMathLibrary.RInterpTo` (`KismetMathLibrary.FindLookAtRotation` (`self.K2_GetActorLocation`) (`self.K2_GetActorLocation` (`GameplayStatics.GetPlayerCharacter` 0))) (struct) 0.0 5.0)))

(fn `UserConstructionScript`
  (`parent.UserConstructionScript`)
  (set `self.Speed` 200.0)
  (set `self.DelayShoot` 1.0))