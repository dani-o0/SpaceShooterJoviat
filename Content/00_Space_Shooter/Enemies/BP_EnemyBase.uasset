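; Base enemy actor for the space shooter that flies in a straight line, fires periodically and damages the player on contact.
; BeginPlay caches the forward vector, and Tick moves the actor along it by Speed without sweeping.
; Tick also accumulates time and calls Fire whenever DelayShoot is exceeded, spawning EnemyBullet at the FirePoint transform.
; Overlapping an SS_Player_Character calls its Damage function, leaving the enemy itself intact.
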(event `self.ReceiveBeginPlay`
  ; Comentario
  (set `self.MovementVector` (`self.GetActorForwardVector`)))

(event `self.ReceiveTick`
  (params (DeltaSeconds :type "Float (single-precision)"))
  ; Comentario
  (`self.K2_SetActorLocation` (+ (`self.K2_GetActorLocation`) (* (* DeltaSeconds (`self.Speed`)) (`self.MovementVector`))))
  (set `self.ShootCurrentTime` (+ (`self.ShootCurrentTime`) DeltaSeconds))
  (if (> (`self.ShootCurrentTime`) (`self.DelayShoot`))
    (`self.Fire`)
    (set `self.ShootCurrentTime` 0.0)))

(event `self.ReceiveActorBeginOverlap`
  (params (OtherActor :type "Actor Object Reference"))
  ; Comentario
  (bind _asss_player_character (cast `/Game/00_Space_Shooter/Player/SS_Player_Character` OtherActor))
  (`/Game/00_Space_Shooter/Player/SS_Player_Character.Damage` _asss_player_character))

(fn `Fire`
  (`|SpawnActorFromClass` "/Game/00_Space_Shooter/Enemies/EnemyBullet.EnemyBullet_C" (`SceneComponent.K2_GetComponentToWorld` (`self.FirePoint`)) "Undefined" "MultiplyWithRoot" null null))

(fn `UserConstructionScript`)