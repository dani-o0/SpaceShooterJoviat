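; Fast enemy variant for the space shooter that moves and fires on a fixed timer.
; Tick moves it along MovementVector at Speed without sweep and accumulates time until DelayShoot is exceeded, then calls Fire and FireTwo and resets the timer.
; FireTwo spawns an EnemyBullet at each of two fire points.
; The construction script runs the parent's, then sets this variant's speed and fire delay.
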(event `self.ReceiveTick`
  (params (DeltaSeconds :type "Float (single-precision)"))
  ; Comentario
  (`self.K2_SetActorLocation` (+ (`self.K2_GetActorLocation`) (* (* DeltaSeconds (`self.Speed`)) (`self.MovementVector`))))
  (set `self.ShootCurrentTime` (+ (`self.ShootCurrentTime`) DeltaSeconds))
  (if (> (`self.ShootCurrentTime`) (`self.DelayShoot`))
    (`self.Fire`)
    (`self.FireTwo`)
    (set `self.ShootCurrentTime` 0.0)))

(fn `FireTwo`
  (`|SpawnActorFromClass` "/Game/00_Space_Shooter/Enemies/EnemyBullet.EnemyBullet_C" (`SceneComponent.K2_GetComponentToWorld` (`self.FirePoint1`)) "Undefined" "MultiplyWithRoot" null null)
  (`|SpawnActorFromClass` "/Game/00_Space_Shooter/Enemies/EnemyBullet.EnemyBullet_C" (`SceneComponent.K2_GetComponentToWorld` (`self.FirePoint2`)) "Undefined" "MultiplyWithRoot" null null))

(fn `UserConstructionScript`
  (`parent.UserConstructionScript`)
  (set `self.Speed` 200.0)
  (set `self.DelayShoot` 0.5))